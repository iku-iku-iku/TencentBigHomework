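; BP_TargetSpawnerGatherer is a gatherer that links gathered Target actors so that hitting one clears the others.
; As each new actor is processed, it updates the gathered list and binds a handler to that Target's first-hit delegate.
; On that hit, the handler loops over the other gathered Targets and, for those with a valid spawner, resets the spawner through their spawn component and destroys them.
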(event `self.ProcessNewGatheredActor`
  (params (Actor :type "Actor Object Reference"))
  (`|ExecutionSequence`
    (:`then_0`
      (`self.UpdateGatheredActors`))
    (:`then_1`
      (bind _astarget (cast `Target` Actor))
      (add `Target.BeHitFirstTimeDelegate` _astarget (delegate `BeHitHandler`)))))

(event `BeHitHandler`
  (params (BeHitTarget :type "Target Object Reference"))
  (for _array_element (`self.GatheredActors`)
    (if (!= BeHitTarget _array_element)
      (bind _astarget (cast `Target` _array_element))
      (bind _returnvalue (`Target.GetSpawnComponent` _astarget))
      (`/Engine/EditorBlueprintResources/StandardMacros.IsValid` (`SpawnComponent.Spawner` _returnvalue)
        (:`Is Valid`
          (`SpawnComponent.ResetSpawner` _returnvalue)
          (`self.K2_DestroyActor` _astarget))))))

(fn `UserConstructionScript`)