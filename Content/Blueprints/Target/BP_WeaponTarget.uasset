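; BP_WeaponTarget is a target that rewards whoever hits it with a random weapon and score.
; Its hit effect event spawns an actor from a random entry in WeaponClasses and hands it to the hitter's player character through a BeObtainedBy interface message.
; It then casts the hitter's state to ScorePlayerState and adds DeltaScore, skipping the score if that cast fails.
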(event `self.EffectWhenHitBy`
  (params (Hitter :type "GunplayPlayerController Object Reference"))
  (set `self.Hitter` null)
  (bind _returnvalue (`|SpawnActorFromClass` (`KismetArrayLibrary.Array_Random` (`self.WeaponClasses`)) (`self.Spawn Transform`) "Undefined" "OverrideRootScale" null null))
  (message `BeObtainedInterface.BeObtainedBy` _returnvalue (`GunplayPlayerController.GetPlayerCharacter` Hitter))
  (bind _asscore_player_state (cast `ScorePlayerState` (`GunplayPlayerController.GetState` Hitter)))
  (`ScorePlayerState.AddScore` _asscore_player_state (`self.DeltaScore`)))

(fn `UserConstructionScript`)