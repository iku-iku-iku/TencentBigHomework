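; HP target that rewards whoever hits it with score and health.
; The EffectwhenHitby event adds DeltaScore to the hitter's ScorePlayerState, then separately raises the HP on the hitter's character StatusComponent by DeltaHP, capped at MaxHP.
; A sequence keeps the two effects independent, so the HP change still runs if the player state cast fails.
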(event `self.EffectWhenHitBy`
  (params (Hitter :type "GunplayPlayerController Object Reference"))
  (bind _statuscomponent (`GunplayCharacter.StatusComponent` (`GunplayPlayerController.GetPlayerCharacter` Hitter)))
  (`|ExecutionSequence`
    (:`then_0`
      (bind _asscore_player_state (cast `ScorePlayerState` (`GunplayPlayerController.GetState` Hitter)))
      (`ScorePlayerState.AddScore` _asscore_player_state (`self.DeltaScore`)))
    (:`then_1`
      (`CharacterStatusComponent.SetHP` _statuscomponent (`KismetMathLibrary.Min` (`CharacterStatusComponent.MaxHP` _statuscomponent) (+ (`CharacterStatusComponent.HP` _statuscomponent) (`self.DeltaHP`)))))))

(fn `UserConstructionScript`)